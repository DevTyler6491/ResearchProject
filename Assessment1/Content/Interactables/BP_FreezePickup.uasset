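; BP_FreezePickup is a collectible that grants the freeze ability to either the top-down player character or an AI.
; On sphere overlap it sets the collector's CanFreeze flag and turns on its point light.
; It then calls SpawnPickup on the level's BP_BoxExtent, found at BeginPlay, and destroys itself.
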(event `self.ReceiveBeginPlay`
  (bind _returnvalue (`GameplayStatics.GetActorOfClass` "/Game/Interactables/BP_BoxExtent.BP_BoxExtent_C"))
  (set `self.BoxExtentRef` _returnvalue))

(event `self.Sphere1.OnComponentBeginOverlap`
  (params (OverlappedComponent :type "PrimitiveComponent Object Reference") (OtherActor :type "Actor Object Reference") (OtherComp :type "PrimitiveComponent Object Reference") (OtherBodyIndex :type Integer) (bFromSweep :type Boolean) (SweepResult :type "HitResult Structure (by ref)"))
  (bind _asbp_top_down_character (cast `/Game/TopDown/Blueprints/BP_TopDownCharacter` OtherActor)
    (:`then`
      (set `/Game/TopDown/Blueprints/BP_TopDownCharacter.CanFreeze` true _asbp_top_down_character)
      (`SceneComponent.SetVisibility` (`/Game/TopDown/Blueprints/BP_TopDownCharacter.PointLight` _asbp_top_down_character) true false))
    (:`CastFailed`
      (bind _asbp_ai (cast `/Game/AI/BP_AI` OtherActor))
      (set `/Game/AI/BP_AI.CanFreeze` true _asbp_ai)
      (`SceneComponent.SetVisibility` (`/Game/AI/BP_AI.PointLight` _asbp_ai) true false)))
  (`/Game/Interactables/BP_BoxExtent.SpawnPickup` (`self.BoxExtentRef`))
  (`self.K2_DestroyActor`))

(fn `UserConstructionScript`)