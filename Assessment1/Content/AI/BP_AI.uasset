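; AI opponent that picks up balls and can freeze the player character or be frozen itself.
; Box overlaps or BallIsWithinRange collect the target ball, up to three, attaching each to a mesh socket with physics off.
; Touching the player while CanFreeze is set freezes them, spending the charge and hiding the light.
; Being frozen stops movement, sets blackboard IsFrozen and toggles ice visibility, toggling back on a timer.
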(event `self.Box.OnComponentBeginOverlap`
  (params (OverlappedComponent :type "PrimitiveComponent Object Reference") (OtherActor :type "Actor Object Reference") (OtherComp :type "PrimitiveComponent Object Reference") (OtherBodyIndex :type Integer) (bFromSweep :type Boolean) (SweepResult :type "HitResult Structure (by ref)"))
  (bind _heldballss (`self.HeldBallss`))
  (bind _targetball (`self.TargetBall`))
  (bind _asbp_ball (cast `/Game/Interactables/BP_Ball` OtherActor)
    (:`then`
      (if (== _asbp_ball _targetball)
        (if (and (< (`self.HeldBallss`) 3) (`/Game/Interactables/BP_Ball.bCanPickup` _targetball)) :!label _label
          (set `/Game/Interactables/BP_Ball.bCanPickup` false _targetball)
          (`KismetArrayLibrary.Array_Set` (`self.BallReference`) (`self.HeldBallss`) _targetball)
          (`/Engine/EditorBlueprintResources/StandardMacros.IncrementInt` _heldballss
            (:`  `
              (`PrimitiveComponent.SetSimulatePhysics` (`/Game/Interactables/BP_Ball.Ball` _targetball) false)
              (switch `int` _heldballss
                (:`1`
                  (set `self.SocketToAttach` "BallSocket"))
                (:`2`
                  (set `self.SocketToAttach` "BallSocket2"))
                (:`3`
                  (set `self.SocketToAttach` "BallSocket3")))
              (`self.K2_AttachToComponent` _targetball (`self.Mesh`) (`self.SocketToAttach`) "SnapToTarget" "KeepRelative" "KeepRelative" true))))))
    (:`CastFailed`
      (bind _asbp_top_down_character (cast `/Game/TopDown/Blueprints/BP_TopDownCharacter` OtherActor))
      (if (`self.CanFreeze`)
        (`/Game/TopDown/Blueprints/BP_TopDownCharacter.Frozen` _asbp_top_down_character)
        (set `self.CanFreeze` false)
        (`SceneComponent.SetVisibility` (`self.PointLight`) false false)))))

(event `BallIsWithinRange`
  (goto _label))

(event `Frozen`
  (`MovementComponent.StopMovementImmediately` (`self.CharacterMovement`))
  (`BlackboardComponent.SetValueAsBool` (`AIBlueprintHelperLibrary.GetBlackboard` null) "IsFrozen" true)
  (`SceneComponent.ToggleVisibility` (`self.Ice`) false)
  (`KismetSystemLibrary.K2_SetTimer` null "ToggleIceVisibility" 5.0))

(event `self.ReceiveBeginPlay`
  (`BlackboardComponent.SetValueAsFloat` (`AIBlueprintHelperLibrary.GetBlackboard` (`AIBlueprintHelperLibrary.GetAIController` self)) "DifficultyLevel" 0.5))

(fn `ToggleIceVisibility`
  (`SceneComponent.ToggleVisibility` (`self.Ice`) false))

(fn `UserConstructionScript`)